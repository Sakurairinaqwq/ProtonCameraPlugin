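; BP_HoverSpring is a scene-component-style raycast suspension spring that pushes a Collider body away from surfaces beneath it.
; Each Tick it traces down its local up axis by Length on the Visibility channel to set Grounded and compression.
; When grounded, it applies a spring-damper force at the impact point, deriving damping from compression change over delta time.
; It also computes WheelLocation from hit distance or full Length, offset by WheelRadius.
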(event `self.ReceiveTick`
  (params (DeltaSeconds :type "Float (single-precision)"))
  (bind _returnvalue (`self.K2_GetComponentLocation`))
  (`/Engine/EditorBlueprintResources/StandardMacros.IsValid` (`self.Collider`)
    (:`Is Valid`
      (bind (_outhit _returnvalue_2) (`KismetSystemLibrary.LineTraceSingle` _returnvalue (- _returnvalue (* (`self.GetUpVector`) (`self.Length`))) "TraceTypeQuery1"))
      (bind _output_get (set `self.bGrounded` _returnvalue_2))
      (if _output_get
        (bind (_bblockinghit _binitialoverlap _time _distance _location _impactpoint) (`GameplayStatics.BreakHitResult` _outhit))
        (bind _returnvalue_3 (- (`self.Length`) _distance))
        (bind _output_get_2 (set `self.dCompression` (`KismetMathLibrary.SafeDivide` (- _returnvalue_3 (`self.compression`)) DeltaSeconds)))
        (bind _output_get_3 (set `self.compression` _returnvalue_3))
        (set `self.compressionRatio` (`KismetMathLibrary.SafeDivide` _output_get_3 (`self.Length`)))
        (`PrimitiveComponent.AddForceAtLocation` (`self.Collider`) (* (`self.GetUpVector`) (+ (* _output_get_2 (`self.DampRate`)) (* _returnvalue_3 (`self.SpringRate`)))) _impactpoint "None"))
      (set `self.wheelLocation` (- (`self.K2_GetComponentLocation`) (* (`self.GetUpVector`) (- (select `bool` _output_get :`false` (`self.Length`) :`true` _distance :!type "Float (double-precision)") (`self.wheelRadius`))))))))