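; Test pawn for a player-flown physics plane with a cycleable ProtonCamera.
; Enhanced Input drives thrust, rudder, elevator and ailerons as mass-independent forces and torques on AVCTestPlane.
; Tick adds axis-driven steering with roll limited by bank angle, plus speed-scaled forces opposing vertical and sideways velocity as simple aerodynamics.
; Three hover springs use the plane as collider and position wheel spheres; look input spins the camera.
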(event `EnhancedInput|/ProtonCameraPlugin/TestPawns/Input/IA_Throttle`
  (params (ActionValue :type "Float (double-precision)") (ElapsedSeconds :type "Float (double-precision)") (TriggeredSeconds :type "Float (double-precision)") (InputAction :type "InputAction Object Reference" :default "/ProtonCameraPlugin/TestPawns/Input/IA_Throttle.IA_Throttle"))
  ;[0.01873 0.391 1] Thrust
  (:`Triggered`
    (`PrimitiveComponent.AddForce` (`self.AVCTestPlane`) (* ActionValue 1000.0 (`self.GetActorForwardVector`)) "None" true)))

(event `EnhancedInput|/ProtonCameraPlugin/TestPawns/Input/IA_Rudder`
  (params (ActionValue :type "Float (double-precision)") (ElapsedSeconds :type "Float (double-precision)") (TriggeredSeconds :type "Float (double-precision)") (InputAction :type "InputAction Object Reference" :default "/ProtonCameraPlugin/TestPawns/Input/IA_Rudder.IA_Rudder"))
  ;[0.6771 0.08463 0.08463] Rudder
  (:`Triggered`
    (`PrimitiveComponent.AddTorqueInRadians` (`self.AVCTestPlane`) (* ActionValue 0.6 (`self.GetActorUpVector`)) "None" true)))

(event `self.ReceiveBeginPlay`
  (`EnhancedInputSubsystemInterface.AddMappingContext` (pcsubsystem `EnhancedInputLocalPlayerSubsystem` (`GameplayStatics.GetPlayerController` 0)) "/ProtonCameraPlugin/TestPawns/Input/IMC_Default.IMC_Default" 0 (struct)))

(event `EnhancedInput|/ProtonCameraPlugin/TestPawns/Input/IA_Elevator`
  (params (ActionValue :type "Float (double-precision)") (ElapsedSeconds :type "Float (double-precision)") (TriggeredSeconds :type "Float (double-precision)") (InputAction :type "InputAction Object Reference" :default "/ProtonCameraPlugin/TestPawns/Input/IA_Elevator.IA_Elevator"))
  ;[1 0.2379 0.02717] Elevator
  (:`Triggered`
    (`PrimitiveComponent.AddTorqueInRadians` (`self.AVCTestPlane`) (* ActionValue 1.6 (`self.GetActorRightVector`)) "None" true)))

(event `self.ReceiveTick`
  (params (DeltaSeconds :type "Float (single-precision)"))
  (bind _returnvalue (`self.GetActorUpVector`))
  (bind _returnvalue_2 (`self.GetActorRightVector`))
  (bind _returnvalue_roll (`KismetMathLibrary.BreakRotator` (`self.K2_GetActorRotation`)))
  (bind _returnvalue_3 (`self.GetInputAxisKeyValue`))
  (bind _avctestplane (`self.AVCTestPlane`))
  (`PrimitiveComponent.AddTorqueInRadians` (`self.AVCTestPlane`) (+ (* (`self.GetInputAxisKeyValue`) 1.2 (`self.GetActorUpVector`)) (* (`self.GetInputAxisKeyValue`) -2.2 (`self.GetActorRightVector`)) (* _returnvalue_3 (`KismetMathLibrary.SelectFloat` 0.0 -3.0 (and (== (`KismetMathLibrary.SignOfFloat` _returnvalue_3) (`KismetMathLibrary.SignOfFloat` _returnvalue_roll)) (> (`KismetMathLibrary.Abs` _returnvalue_roll) 6.0))) (`self.GetActorForwardVector`))) "None" true)
  ;[0 0.6771 0.3449] Aerodynamics
  (bind _returnvalue_4 (`PrimitiveComponent.GetPhysicsLinearVelocity` _avctestplane "None"))
  (bind _returnvalue_5 (`KismetMathLibrary.MapRangeUnclamped` (`KismetMathLibrary.VSize` _returnvalue_4) 0.0 5000.0 0.0 1.0))
  (`PrimitiveComponent.AddForce` _avctestplane (+ (* _returnvalue (`KismetMathLibrary.Dot_VectorVector` _returnvalue _returnvalue_4) -3.0 _returnvalue_5) (* _returnvalue_2 (`KismetMathLibrary.Dot_VectorVector` _returnvalue_4 _returnvalue_2) -15.0 _returnvalue_5)) "None" true)
  (`SceneComponent.K2_SetWorldLocation` (`self.Sphere2`) (`/ProtonCameraPlugin/TestPawns/BP_HoverSpring.wheelLocation` (`self.BP_HoverSpringF`)) false false)
  (`SceneComponent.K2_SetWorldLocation` (`self.Sphere1`) (`/ProtonCameraPlugin/TestPawns/BP_HoverSpring.wheelLocation` (`self.BP_HoverSpringL`)) false false)
  (`SceneComponent.K2_SetWorldLocation` (`self.Sphere`) (`/ProtonCameraPlugin/TestPawns/BP_HoverSpring.wheelLocation` (`self.BP_HoverSpringR`)) false false)
  (`ProtonCameraComponent.AddManualSpinXY` (`self.ProtonCamera`) (`KismetMathLibrary.MakeVector2D` (`|GetInputActionValue`) (`|GetInputActionValue`)) false))

(event `EnhancedInput|/ProtonCameraPlugin/TestPawns/Input/IA_Ailerons`
  (params (ActionValue :type "Float (double-precision)") (ElapsedSeconds :type "Float (double-precision)") (TriggeredSeconds :type "Float (double-precision)") (InputAction :type "InputAction Object Reference" :default "/ProtonCameraPlugin/TestPawns/Input/IA_Ailerons.IA_Ailerons"))
  ;[1 0.4074 0] Ailerons
  (:`Triggered`
    (`PrimitiveComponent.AddTorqueInRadians` (`self.AVCTestPlane`) (* (`self.GetActorForwardVector`) -2.5 ActionValue) "None" true)))

(event `EnhancedInput|/ProtonCameraPlugin/TestPawns/Input/IA_ChangeCamera`
  (params (ActionValue :type Boolean) (ElapsedSeconds :type "Float (double-precision)") (TriggeredSeconds :type "Float (double-precision)") (InputAction :type "InputAction Object Reference" :default "/ProtonCameraPlugin/TestPawns/Input/IA_ChangeCamera.IA_ChangeCamera"))
  (:`Started`
    (`ProtonCameraComponent.CycleCameraProfile` (`self.ProtonCamera`))))

(fn `UserConstructionScript`
  (bind _avctestplane (`self.AVCTestPlane`))
  (set `/ProtonCameraPlugin/TestPawns/BP_HoverSpring.Collider` _avctestplane (`self.BP_HoverSpringF`))
  (set `/ProtonCameraPlugin/TestPawns/BP_HoverSpring.Collider` _avctestplane (`self.BP_HoverSpringL`))
  (set `/ProtonCameraPlugin/TestPawns/BP_HoverSpring.Collider` _avctestplane (`self.BP_HoverSpringR`)))