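; BP_PCCar is a physics-driven test car pawn on four hover springs, with a ProtonCamera follow camera.
; Grounded rear springs apply throttle force that tapers near top speed, while steering adds yaw torque signed by travel direction.
; Tick applies speed- and compression-scaled lateral grip, biased rearward, and lerps sphere wheels to spring locations.
; The camera takes spin and mouse input, cycles profiles and switches to reverse view when moving backward.
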(event `EnhancedInput|/ProtonCameraPlugin/TestPawns/Input/IA_Throttle`
  (params (ActionValue :type "Float (double-precision)") (ElapsedSeconds :type "Float (double-precision)") (TriggeredSeconds :type "Float (double-precision)") (InputAction :type "InputAction Object Reference" :default "/ProtonCameraPlugin/TestPawns/Input/IA_Throttle.IA_Throttle"))
  ;[0.01873 0.391 1] Thrust
  (:`Triggered`
    (for (_array_element _array_index) (`self.Array`)
      (if (and (> _array_index 1) (`/ProtonCameraPlugin/TestPawns/BP_HoverSpring.bGrounded` _array_element))
        (`PrimitiveComponent.AddForceAtLocation` (`self.AVCTestCar`) (* (* ActionValue 250000.0 (`self.GetActorForwardVector`)) (`KismetMathLibrary.MapRangeClamped` (* (`KismetMathLibrary.VSize` (`self.GetVelocity`)) 0.01) 40.0 45.0 1.0)) (`/ProtonCameraPlugin/TestPawns/BP_HoverSpring.wheelLocation` _array_element) "None")))))

(event `EnhancedInput|/ProtonCameraPlugin/TestPawns/Input/IA_Ailerons`
  (params (ActionValue :type "Float (double-precision)") (ElapsedSeconds :type "Float (double-precision)") (TriggeredSeconds :type "Float (double-precision)") (InputAction :type "InputAction Object Reference" :default "/ProtonCameraPlugin/TestPawns/Input/IA_Ailerons.IA_Ailerons"))
  ;[0.6771 0.08463 0.08463] Steering
  (:`Triggered`
    (`PrimitiveComponent.AddTorqueInRadians` (`self.AVCTestCar`) (* ActionValue 2.0 (`self.GetActorUpVector`) (`KismetMathLibrary.SignOfFloat` (`KismetMathLibrary.Dot_VectorVector` (`self.GetActorForwardVector`) (`self.GetVelocity`)))) "None" true)))

(event `self.ReceiveBeginPlay`
  (`EnhancedInputSubsystemInterface.AddMappingContext` (pcsubsystem `EnhancedInputLocalPlayerSubsystem` (`GameplayStatics.GetPlayerController` 0)) "/ProtonCameraPlugin/TestPawns/Input/IMC_Default.IMC_Default" 0 (struct)))

(event `self.ReceiveTick`
  (params (DeltaSeconds :type "Float (single-precision)"))
  (bind _returnvalue (`self.GetActorRightVector`))
  (bind _avctestcar (`self.AVCTestCar`))
  (bind _mousespeed (`self.MouseSpeed`))
  (bind _localvelocity_x (`KismetMathLibrary.BreakVector` (`ProtonCameraComponent.LocalVelocity` (`self.ProtonCamera`))))
  (`|ExecutionSequence`
    (:`then_0`
      ;[1 0.2242 0.04393] Adding Forces
      (bind _returnvalue_2 (`PrimitiveComponent.GetPhysicsLinearVelocity` _avctestcar "None"))
      (for (_array_element _array_index) (`self.Array`)
        (if (`/ProtonCameraPlugin/TestPawns/BP_HoverSpring.bGrounded` _array_element)
          (`PrimitiveComponent.AddForceAtLocation` _avctestcar (* _returnvalue (`KismetMathLibrary.FClamp` (`KismetMathLibrary.Dot_VectorVector` _returnvalue_2 _returnvalue) -400.0 400.0) -6000.0 (`KismetMathLibrary.MapRangeUnclamped` (`KismetMathLibrary.VSize` _returnvalue_2) 0.0 3000.0 1.0 0.4) (`KismetMathLibrary.MultiplyMultiply_FloatFloat` (`/ProtonCameraPlugin/TestPawns/BP_HoverSpring.compressionRatio` _array_element) 0.75) (`KismetMathLibrary.SelectFloat` 1.0 1.3 (> _array_index 1))) (`/ProtonCameraPlugin/TestPawns/BP_HoverSpring.wheelLocation` _array_element) "None"))))
    (:`then_1`
      ;[1 0.07011 0.22] Set Wheel Positions
      (for (_array_element_2 _array_index_2) (`self.Array_0`)
        (`SceneComponent.K2_SetWorldLocation` _array_element_2 (`KismetMathLibrary.VLerp` (`SceneComponent.K2_GetComponentLocation` _array_element_2) (+ (* _returnvalue_2 0.008) (`/ProtonCameraPlugin/TestPawns/BP_HoverSpring.wheelLocation` (`|GetArrayItem` (`self.Array`) _array_index_2))) (* DeltaSeconds 30.0)) false false)
        ;[1 0.6533 0.007625] Spin Camera
        (`ProtonCameraComponent.AddManualSpinXY` (`self.ProtonCamera`) (`KismetMathLibrary.MakeVector2D` (`|GetInputActionValue`) (`|GetInputActionValue`)) false)))
    (:`then_2`
      ;[0.3147 0.2448 1] Mouse Control
      (bind _output_get (set `self.MouseCacheX` (+ (`self.MouseCacheX`) (* (`self.GetInputAxisKeyValue`) _mousespeed))))
      (bind _output_get_2 (set `self.MouseCacheY` (`KismetMathLibrary.FClamp` (+ (`self.MouseCacheY`) (* (`self.GetInputAxisKeyValue`) _mousespeed)) -80.0 15.0)))
      (`ProtonCameraComponent.AddManualRotation` (`self.ProtonCamera`) (`KismetMathLibrary.MakeRotator` 0.0 _output_get_2 _output_get) false)
      (`ProtonCameraComponent.SetIntoReverse` (`self.ProtonCamera`) (< (`KismetMathLibrary.SignOfFloat` (+ _localvelocity_x 1.0)) 0.0)))))

(event `EnhancedInput|/ProtonCameraPlugin/TestPawns/Input/IA_ChangeCamera`
  (params (ActionValue :type Boolean) (ElapsedSeconds :type "Float (double-precision)") (TriggeredSeconds :type "Float (double-precision)") (InputAction :type "InputAction Object Reference" :default "/ProtonCameraPlugin/TestPawns/Input/IA_ChangeCamera.IA_ChangeCamera"))
  ;[0.9417 0.05898 1] Change Camera
  (:`Triggered`
    (`ProtonCameraComponent.CycleCameraProfile` (`self.ProtonCamera`))))

(fn `UserConstructionScript`
  (bind _bp_hoverspringfl (`self.BP_HoverSpringFL`))
  (bind _bp_hoverspringfr (`self.BP_HoverSpringFR`))
  (bind _avctestcar (`self.AVCTestCar`))
  (bind _bp_hoverspringrl (`self.BP_HoverSpringRL`))
  (bind _bp_hoverspringrr (`self.BP_HoverSpringRR`))
  (set `/ProtonCameraPlugin/TestPawns/BP_HoverSpring.Collider` _avctestcar _bp_hoverspringfl)
  (set `/ProtonCameraPlugin/TestPawns/BP_HoverSpring.Collider` _avctestcar _bp_hoverspringfr)
  (set `/ProtonCameraPlugin/TestPawns/BP_HoverSpring.Collider` _avctestcar _bp_hoverspringrl)
  (set `/ProtonCameraPlugin/TestPawns/BP_HoverSpring.Collider` _avctestcar _bp_hoverspringrr)
  (set `self.Array` (`|MakeArray` _bp_hoverspringfl _bp_hoverspringfr _bp_hoverspringrl _bp_hoverspringrr))
  (set `self.Array_0` (`|MakeArray` (`self.SphereFL`) (`self.SphereFR`) (`self.SphereRL`) (`self.SphereRR`))))